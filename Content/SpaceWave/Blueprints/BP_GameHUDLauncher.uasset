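; Level actor that shows the SpaceWave game HUD and watches for the end of the match.
; On BeginPlay it creates the BP_GameHUD widget and adds it to the viewport.
; Each Tick it searches for PlayerShip actors, treating none left as a loss and a set IsGameEnds flag as a win.
; Either outcome saves the team score and result to MyGameInstance, then opens the AH_Ranking level.
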(event EventBeginPlay
  (bind _returnvalue (UserInterface|CreateWidget "/Game/SpaceWave/Blueprints/BP_GameHUD.BP_GameHUD_C"))
  (bind _output_get (Variables|Default|SetHUD _returnvalue))
  (UserInterface|Viewport|AddtoViewport _output_get 0))

(event Collision|EventActorBeginOverlap
  (params (OtherActor :type Actor%20Object%20Reference)))

(event EventTick
  (params (DeltaSeconds :type Float%20%28single-precision%29))
  ;[1 1 1] Check loose game
  (bind _outactors (Actor|GetAllActorsOfClass "/Script/AeroHero.PlayerShip"))
  (if (== (Utilities|Array|Length _outactors) 0)
    (Variables|Default|SetplayerWins false)
    ;[1 1 1] Save on game instance
    (bind _asmy_game_instance (Utilities|Casting|CastToMyGameInstance (Game|GetGameInstance) :!label _label))
    (Variables|/Game/SpaceWave/Blueprints/MyGameInstance.MyGameInstance_C|SetCurrentScoreGI _asmy_game_instance (Variables|Default|GetcurrentTeamScore))
    (Variables|/Game/SpaceWave/Blueprints/MyGameInstance.MyGameInstance_C|SetIsPlayerWinsGI _asmy_game_instance (Variables|Default|GetplayerWins))
    (Game|OpenLevel(byName) "AH_Ranking")
    (else
      ;[1 1 1] Player finished and wins game
      (if (Variables|Default|GetisGameEnds)
        (Variables|Default|SetplayerWins true)
        (goto _label)))))

(fn ConstructionScript)