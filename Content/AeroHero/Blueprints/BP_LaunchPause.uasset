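; BP_LaunchPause is a Blueprint meant to toggle game pause from player input.
; Middle mouse, Enter and the gamepad special-right button share one path that flips a Paused flag and applies SetGamePaused.
; On pause it creates and displays a BP_PauseHUD widget; nothing here removes it on unpause.
; An author note says this logic malfunctions here and is copied into the Level Blueprint.
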(event EventBeginPlay)

(event Collision|EventActorBeginOverlap
  (params (OtherActor :type Actor%20Object%20Reference)))

(event EventTick
  (params (DeltaSeconds :type Float%20%28single-precision%29)))

(event Input|KeyboardEvents|Enter
  (params (Key :type Key%20Structure))
  ;[1 1 1] NOTE: THIS DOESN'T WORKS FINE IN THIS BLUEPRINT, SO IT'S COPY&PASTE TO LEVEL BLUEPRINT.
  (:Pressed
    (bind _output_get (Variables|Default|SetbPaused (not (Variables|Default|GetbPaused))))
    (Game|SetGamePaused _output_get)
    (if (Variables|Default|GetbPaused)
      (bind _returnvalue (UserInterface|CreateWidget "/Game/AeroHero/Blueprints/BP_PauseHUD.BP_PauseHUD_C"))
      (bind _output_get_2 (Variables|Default|SetPauseHUD _returnvalue))
      (UserInterface|Viewport|AddtoViewport _output_get_2 0))))

(event Input|GamepadEvents|GamepadSpecialRight
  (params (Key :type Key%20Structure))
  ;[1 1 1] NOTE: THIS DOESN'T WORKS FINE IN THIS BLUEPRINT, SO IT'S COPY&PASTE TO LEVEL BLUEPRINT.
  (:Pressed
    (bind _output_get (Variables|Default|SetbPaused (not (Variables|Default|GetbPaused))))
    (Game|SetGamePaused _output_get)
    (if (Variables|Default|GetbPaused)
      (bind _returnvalue (UserInterface|CreateWidget "/Game/AeroHero/Blueprints/BP_PauseHUD.BP_PauseHUD_C"))
      (bind _output_get_2 (Variables|Default|SetPauseHUD _returnvalue))
      (UserInterface|Viewport|AddtoViewport _output_get_2 0))))

(event Input|MouseEvents|MiddleMouseButton
  (params (Key :type Key%20Structure))
  ;[1 1 1] NOTE: THIS DOESN'T WORKS FINE IN THIS BLUEPRINT, SO IT'S COPY&PASTE TO LEVEL BLUEPRINT.
  (:Pressed
    (bind _output_get (Variables|Default|SetbPaused (not (Variables|Default|GetbPaused))))
    (Game|SetGamePaused _output_get)
    (if (Variables|Default|GetbPaused)
      (bind _returnvalue (UserInterface|CreateWidget "/Game/AeroHero/Blueprints/BP_PauseHUD.BP_PauseHUD_C"))
      (bind _output_get_2 (Variables|Default|SetPauseHUD _returnvalue))
      (UserInterface|Viewport|AddtoViewport _output_get_2 0))))

(fn ConstructionScript)